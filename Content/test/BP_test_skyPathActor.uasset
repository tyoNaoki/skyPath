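; Test actor for the SkyPath 3D pathfinding system that previews a path from its location to a local-space test goal.
; When IsDraw is set, the construction script loads sparse voxel octree data and searches voxels, then refines the result through funnel, visibility-shortcut and clothoid spline passes.
; It draws the voxels, shortcut points, spline points and search nodes as debug shapes, with the arrow's rotation feeding the spline.
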(event `self.ReceiveTick`
  (params (DeltaSeconds :type "Float (single-precision)")))

(fn `getGoalLocation`
  (returns (ReturnValue :type "Vector Structure"))
  (return (0.0 0.0 0.0)))

(fn `getMiddleAngleTest`
  (params (angle1 :type "Float (double-precision)") (angle2 :type "Float (double-precision)"))
  (locals (angle1_2D :type "Float (double-precision)") (angle2_2D :type "Float (double-precision)"))
  (bind _angle2 (`local.angle2`))
  (bind _angle1 (`local.angle1`))
  (bind _returnvalue (`SkyPathComponent.getMiddleAngle` (`self.SkyPath`) angle1 angle2))
  (`KismetSystemLibrary.PrintString` (`KismetStringLibrary.Concat_StrStr` "getMiddleAngle : " (`KismetStringLibrary.Conv_DoubleToString` _returnvalue)))
  (if (not (>= _angle1 0.0))
    (set `local.angle1_2D` (+ 360.0 _angle1)))
  (if (not (>= _angle2 0.0))
    (set `local.angle2_2D` (+ 360.0 _angle2)))
  (`KismetSystemLibrary.PrintString` (`KismetStringLibrary.Concat_StrStr` "getMiddleAngle_New : ")))

(fn `getStartLocation`
  (returns (ReturnValue :type "Vector Structure"))
  (return (`SceneComponent.K2_GetComponentLocation` (`self.start_waypoint`))))

(fn `UserConstructionScript`
  (locals (NewLocalVar_0 :type "Array of Vector Structure") (`a*AlgorithmPaths` :type "Array of VoxelData Structure") (funnelAlgorithmPaths :type "Array of Vector Structure") (shortcutPaths :type "Array of Vector Structure") (NewLocalVar_4 :type "Array of Vector Structure") (lineStartLoc :type "Vector Structure") (temp_goalLocation :type "Vector Structure" :default (0.0 0.0 0.0)) (NewLocalVar_5 :type "Vector Structure"))
  (bind _skypath (`self.SkyPath`))
  (bind _returnvalue (`KismetMathLibrary.TransformLocation` (`self.GetTransform`) (`self.test_goalLocation`)))
  (`SceneComponent.K2_SetWorldRotation` (`self.Arrow`) (`self.debug_currentRotation`) false false)
  (if (`self.isDraw`)
    (set `self.isDraw` false)
    (`SceneComponent.K2_SetWorldLocation` (`self.goal_waypoint`) _returnvalue false true)
    (set `local.temp_goalLocation` _returnvalue)
    (bind _returnvalue_2 (`SkyPathComponent.Read_svoData` _skypath (`self.svoName`) 0))
    (if _returnvalue_2
      (bind _returnvalue_3 (`SkyPathComponent.searchVoxels` _skypath (`self.K2_GetActorLocation`) (`local.temp_goalLocation`)))
      (if (!= (`KismetArrayLibrary.Array_Length` _returnvalue_3) 0)
        (bind _output_get (set `local.a*AlgorithmPaths` _returnvalue_3))
        (bind _returnvalue_4 (`SkyPathComponent.GetFunnelAlgorithmResult` _skypath 0.0 _output_get))
        (bind _output_get_2 (set `local.funnelAlgorithmPaths` _returnvalue_4))
        (bind _returnvalue_5 (`SkyPathComponent.GetshortcutPathResult` (`self.SkyPath`) _output_get_2 "ECC_Visibility"))
        (bind _output_get_3 (set `local.shortcutPaths` _returnvalue_5))
        (for (_array_element _array_index) _output_get_3
          (`KismetSystemLibrary.PrintString` (`KismetStringLibrary.Concat_StrStr` "[" (`KismetStringLibrary.Conv_IntToString` _array_index) "] : " (`KismetStringLibrary.Conv_VectorToString` _array_element))))
        (for _array_element_2 (`local.a*AlgorithmPaths`)
          (`KismetSystemLibrary.DrawDebugBox` (break `VoxelData` _array_element_2) (`.extent` (break `VoxelData` _array_element_2)) (struct :`R` 0.054995 :`G` 0.963542 :`B` 0.268576 :`A` 1.0) (struct) 5.0 10.0))
        (for _array_element_3 _output_get_3
          (`KismetSystemLibrary.DrawDebugPoint` _array_element_3 20.0 (struct :`A` 1.0) 5.0))
        (bind _returnvalue_6 (`SkyPathComponent.calcClothoidSplineV2` (`self.SkyPath`) _output_get_3 true (`self.debug_currentRotation`)))
        (for _array_element_4 _returnvalue_6
          (`KismetSystemLibrary.DrawDebugPoint` _array_element_4 10.0 (struct :`R` 0.899306 :`B` 0.229313 :`A` 1.0) 5.0))
        (`SkyPathComponent.drawSeachNodes` (`self.SkyPath`) 0)))))