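; Test actor that exercises a recursive function containing a for loop, run from the construction script.
; Setting the boolean NewVar0 acts as a one-shot trigger: the script clears it and calls TestFunction at index zero.
; TestFunction loops over a small fixed range, prints the array index and value on a match in NewVar1, then recurses to the next index.
; The event graph holds only disabled default events.
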(fn `testFunction`
  (params (NewParam :type Integer))
  (locals (NewLocalVar_0 :type Integer))
  (bind _newvar_1 (`self.NewVar_1`))
  (for _index (range 3)
    (if (`KismetArrayLibrary.Array_IsValidIndex` _newvar_1 NewParam)
      (if (== (`|GetArrayItem` _newvar_1 NewParam) _index)
        (`KismetSystemLibrary.PrintString` (`KismetStringLibrary.Concat_StrStr` (`KismetStringLibrary.Conv_IntToString` NewParam) " : " (`KismetStringLibrary.Conv_IntToString` _index)))
        (`self.testFunction` (+ NewParam 1)))))
  (return))

(fn `UserConstructionScript`
  (if (`self.NewVar_0`)
    (set `self.NewVar_0` false)
    (`self.testFunction` 0)))