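; Flying agent that endlessly roams to random points within an SVO volume along smooth clothoid splines.
; SkyPath searches sparse-octree voxels, then applies funnel, shortcut and clothoid passes; unblocked goals skip straight to the clothoid.
; Tick advances along the current spline, banking from yaw change, and nearing its end builds the next spline from that endpoint, swapping on arrival.
; The initial path always uses voxel search, seeded with the actor's rotation.
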(event `self.ReceiveBeginPlay`
  (bind _returnvalue (`self.onInitializeSpline`))
  (if _returnvalue
    (set `self.start` true)))

(event `self.ReceiveTick`
  (params (DeltaSeconds :type "Float (single-precision)"))
  (set `SkyPathComponent.currentRotation` (`self.K2_GetActorRotation`) (`self.SkyPath1`))
  (if (and (`self.start`) (not (`self.change`)))
    (if (not (`self.stop`))
      (`self.calcMoveDistance` DeltaSeconds))
    (if (and (`self.IsNearGoal` 1000.0) (not (`self.update`)) (not (`self.change`)))
      (set `self.stop` true)
      (set `self.update` true)
      (`self.setStartLocationOnSkyPath`)
      (bind _returnvalue (`self.onSearchSkyPath`))
      (if _returnvalue
        (`self.updatePath`)
        (set `self.stop` false)
        (else
          (set `self.update` false)))
      (elif (and (`self.onArrived`) (`self.update`) (not (`self.change`)))
        (set `self.stop` true)
        (set `self.change` true)
        (`self.onChangeSpline`)
        (set `self.stop` false)
        (set `self.update` false)
        (set `self.change` false)
        (else
          (`self.skyMovement`))))))

(fn `calcMoveDistance`
  (params (deltaTime :type "Float (double-precision)"))
  (set `self.MoveDis` (+ (`self.MoveDis`) (* (`self.mveSpeed`) deltaTime)))
  (return))

(fn `getHitAction`
  (returns (hit :type Boolean))
  (return (`self.hit`)))

(fn `getTargetLocation`
  (returns (nextLocation :type "Vector Structure"))
  (return (`self.nextLocation`)))

(fn `IsNearGoal`
  (params (nearLength :type "Float (double-precision)"))
  (returns (ReturnValue :type Boolean))
  (bind _spline (`self.spline`))
  (if (`KismetSystemLibrary.IsValid` _spline)
    (if (< (`/Game/BP_Spline.calcDistanceToNextLocation` _spline (`self.MoveDis`)) nearLength)
      (return true)
      (else
        _)))
  (return false))

(fn `onArrived`
  (returns (ReturnValue :type Boolean))
  (bind _spline (`self.spline`))
  (if (`KismetSystemLibrary.IsValid` _spline)
    (if (`/Game/BP_Spline.isArrived` _spline (`self.MoveDis`))
      (return true)
      (else
        _)))
  (return false))

(fn `onChangeSpline`
  (set `self.MoveDis` 0.0)
  (`/Game/BP_Spline.changeSpline` (`self.spline`)))

(fn `onInitializeSpline`
  (returns (ReturnValue :type Boolean))
  (bind _spline (`self.spline`))
  (if (not (`/Game/BP_Spline.initiaze` _spline))
    (`self.setStartLocationOnInitialize`)
    (bind _returnvalue (`self.onSearchSkyPath_Initialize`))
    (if _returnvalue
      (`self.updatePath`)
      (`self.onChangeSpline`)
      (set `/Game/BP_Spline.initiaze` true _spline)
      (return true)
      (else
        (return false)))))

(fn `onSearchSkyPath`
  (returns (ReturnValue :type Boolean))
  (bind _startlocation (`self.startLocation`))
  (bind _nextlocation (`self.nextLocation`))
  (`self.setRandomLocation`)
  (bind _outhit (`KismetSystemLibrary.LineTraceSingle` (`self.K2_GetActorLocation`) (`self.nextLocation`) "TraceTypeQuery1"))
  (if (`GameplayStatics.BreakHitResult` _outhit)
    (bind _returnvalue (`self.searchSkyPath` _startlocation _nextlocation))
    (return _returnvalue)
    (else
      (bind _returnvalue_2 (`self.searchClothoidPath` _startlocation _nextlocation))
      (return _returnvalue_2))))

(fn `onSearchSkyPath_Initialize`
  (returns (ReturnValue :type Boolean))
  (`self.setRandomLocation`)
  (bind _returnvalue (`self.searchSkyPath_custom` (`self.startLocation`) (`self.nextLocation`)))
  (return _returnvalue))

(fn `searchClothoidPath`
  (params (startLocation :type "Vector Structure") (goalLocation :type "Vector Structure"))
  (returns (returnValue :type Boolean))
  (bind _array (`|MakeArray` startLocation goalLocation))
  (bind _skypath1 (`self.SkyPath1`))
  (`KismetSystemLibrary.DrawDebugPoint` startLocation 20.0 (struct :`R` 1.0 :`G` 0.466415 :`B` 0.018515 :`A` 1.0) 1.0)
  (`KismetSystemLibrary.DrawDebugPoint` goalLocation 20.0 (struct :`G` 0.217062 :`B` 0.875 :`A` 1.0) 1.0)
  (if false
    (bind _returnvalue (`SkyPathComponent.calcClothoidSpline` _skypath1 _array))
    (set `self.skyPathResult` _returnvalue)
    (else
      (bind _returnvalue_2 (`SkyPathComponent.calcClothoidSplineV2` :`self` _skypath1 :`pathDatas` _array))
      (set `self.skyPathResult` _returnvalue_2)))
  (if (!= (`KismetArrayLibrary.Array_Length` (`self.skyPathResult`)) 0)
    (if (not (not (`self.drawSkyPath`)))
      (for _array_element (`self.skyPathResult`)
        (`KismetSystemLibrary.DrawDebugPoint` _array_element 5.0 (struct :`R` 1.0 :`A` 1.0) 5.0)))
    (return true)
    (else
      (`KismetArrayLibrary.Array_Clear` (`self.skyPathResult`))
      (return false))))

(fn `searchSkyPath`
  (params (StartLocation :type "Vector Structure") (GoalLocaion :type "Vector Structure"))
  (returns (ReturnValue :type Boolean))
  (bind _skypath1 (`self.SkyPath1`))
  (`KismetSystemLibrary.DrawDebugPoint` StartLocation 20.0 (struct :`R` 1.0 :`G` 0.466415 :`B` 0.018515 :`A` 1.0) 5.0)
  (`KismetSystemLibrary.DrawDebugPoint` GoalLocaion 20.0 (struct :`G` 0.217062 :`B` 0.875 :`A` 1.0) 5.0)
  (if (`KismetSystemLibrary.IsValid` _skypath1)
    (bind _returnvalue (`SkyPathComponent.Read_svoData` _skypath1 "svo00" 0))
    (if _returnvalue
      (bind _returnvalue_2 (`SkyPathComponent.searchVoxels` _skypath1 StartLocation GoalLocaion))
      (if (!= (`KismetArrayLibrary.Array_Length` _returnvalue_2) 0)
        (bind _returnvalue_3 (`SkyPathComponent.GetFunnelAlgorithmResult` _skypath1 0.0 _returnvalue_2))
        (bind _returnvalue_4 (`SkyPathComponent.GetshortcutPathResult` (`self.SkyPath1`) _returnvalue_3 "ECC_WorldStatic"))
        (bind _returnvalue_5 (`SkyPathComponent.calcClothoidSplineV2` :`self` (`self.SkyPath1`) :`pathDatas` _returnvalue_4))
        (if (!= (`KismetArrayLibrary.Array_Length` _returnvalue_5) 0)
          (set `self.skyPathResult` _returnvalue_5)
          (if (not (not (`self.drawSkyPath`)))
            (for _array_element (`self.skyPathResult`)
              (`KismetSystemLibrary.DrawDebugPoint` _array_element 5.0 (struct :`R` 1.0 :`A` 1.0) 5.0)))
          (return true)
          (else
            _)))))
  (`KismetArrayLibrary.Array_Clear` (`self.skyPathResult`))
  (return false))

(fn `searchSkyPath_custom`
  (params (StartLocation :type "Vector Structure") (GoalLocaion :type "Vector Structure"))
  (returns (ReturnValue :type Boolean))
  (bind _skypath1 (`self.SkyPath1`))
  (`KismetSystemLibrary.DrawDebugPoint` StartLocation 20.0 (struct :`R` 1.0 :`G` 0.466415 :`B` 0.018515 :`A` 1.0) 5.0)
  (`KismetSystemLibrary.DrawDebugPoint` GoalLocaion 20.0 (struct :`G` 0.217062 :`B` 0.875 :`A` 1.0) 5.0)
  (if (`KismetSystemLibrary.IsValid` _skypath1)
    (bind _returnvalue (`SkyPathComponent.Read_svoData` _skypath1 "svo00" 0))
    (if _returnvalue
      (bind _returnvalue_2 (`SkyPathComponent.searchVoxels` _skypath1 StartLocation GoalLocaion))
      (if (!= (`KismetArrayLibrary.Array_Length` _returnvalue_2) 0)
        (bind _returnvalue_3 (`SkyPathComponent.GetFunnelAlgorithmResult` _skypath1 0.0 _returnvalue_2))
        (bind _returnvalue_4 (`SkyPathComponent.GetshortcutPathResult` (`self.SkyPath1`) _returnvalue_3 "ECC_WorldStatic"))
        (bind _returnvalue_5 (`SkyPathComponent.calcClothoidSplineV2` (`self.SkyPath1`) _returnvalue_4 true (`self.K2_GetActorRotation`)))
        (if (!= (`KismetArrayLibrary.Array_Length` _returnvalue_5) 0)
          (set `self.skyPathResult` _returnvalue_5)
          (if (not (not (`self.drawSkyPath`)))
            (for _array_element (`self.skyPathResult`)
              (`KismetSystemLibrary.DrawDebugPoint` _array_element 5.0 (struct :`R` 1.0 :`A` 1.0) 5.0)))
          (return true)
          (else
            _)))))
  (`KismetArrayLibrary.Array_Clear` (`self.skyPathResult`))
  (return false))

(fn `setRandomLocation`
  (bind _svovolume (`self.svoVolume`))
  (bind _maxtargetrange (`self.maxTargetRange`))
  (bind (_origin _boxextent) (`self.GetActorBounds` _svovolume false))
  (bind (_returnvalue_x _returnvalue_y) (`KismetMathLibrary.BreakVector` (`KismetMathLibrary.RandomPointInBoundingBox` _origin _boxextent)))
  (if (`KismetSystemLibrary.IsValid` _svovolume)
    (set `self.nextLocation` (`KismetMathLibrary.MakeVector` _returnvalue_x _returnvalue_y (`KismetMathLibrary.RandomFloatInRange` (`|GetArrayItem` _maxtargetrange) (`|GetArrayItem` _maxtargetrange 1))))
    (return)))

(fn `setStartLocationOnInitialize`
  (set `self.startLocation` (`self.K2_GetActorLocation`))
  (return))

(fn `setStartLocationOnSkyPath`
  (bind _skypathresult (`self.skyPathResult`))
  (set `self.startLocation` (`|GetArrayItem` _skypathresult (`KismetArrayLibrary.Array_LastIndex` _skypathresult)))
  (return))

(fn `setTargetLocation`
  (params (targetLocation :type "Vector Structure"))
  (set `self.nextLocation` targetLocation))

(fn `skyMovement`
  (bind _spline (`self.spline`))
  (bind _movedis (`self.MoveDis`))
  (bind _movedis_2 (`self.MoveDis`))
  (bind _currentspline (`/Game/BP_Spline.currentSpline` (`self.spline`)))
  (if (`/Game/BP_Spline.initiaze` (`self.spline`))
    (if (`KismetSystemLibrary.IsValid` _currentspline)
      (if (<= _movedis (`SplineComponent.GetSplineLength` _currentspline))
        (bind _newparam (`/Game/BP_Spline.GetCurrentLocation` _spline _movedis))
        (bind _returnvalue (`/Game/BP_Spline.GetRotation` _spline _movedis_2))
        (bind _returnvalue_2 (`/Game/BP_Spline.GetNextRotation` _spline _movedis_2 100.0))
        (bind (_returnvalue_roll _returnvalue_pitch _returnvalue_yaw) (`KismetMathLibrary.BreakRotator` (`KismetMathLibrary.NormalizedDeltaRotator` (`KismetMathLibrary.MakeRotator` 0.0 0.0 (.yaw _returnvalue_2)) (`KismetMathLibrary.MakeRotator` 0.0 0.0 (.yaw _returnvalue)))))
        (bind _returnvalue_3 (`KismetMathLibrary.FInterpTo` (`self.currentYaw`) _returnvalue_yaw (`GameplayStatics.GetWorldDeltaSeconds`)))
        (`self.K2_SetActorLocationAndRotation` _newparam (`KismetMathLibrary.MakeRotator` _returnvalue_3 (.pitch _returnvalue_2) (.yaw _returnvalue_2)))
        (set `self.currentYaw` _returnvalue_3)))))

(fn `updatePath`
  (bind _spline (`self.spline`))
  (`/Game/BP_Spline.updateSpline` _spline (`self.skyPathResult`) (`/Game/BP_Spline.getNextSpline` _spline)))

(fn `UserConstructionScript`
  (locals (SkyPath :type "SkyPathComponent Object Reference") (temp_goalLocation :type "Vector Structure") (NewLocalVar_1 :type "Array of  Structure") (NewLocalVar_2 :type "Array of Vector Structure") (NewLocalVar_3 :type "Array of Vector Structure") (NewLocalVar_0 :type "Vector Structure" :default (0.0 0.0 0.0)))
  (bind (_returnvalue_x _returnvalue_y _returnvalue_z) (`KismetMathLibrary.BreakVector` (`self.K2_GetActorLocation`)))
  (set `self.maxTargetRange` (`|MakeArray` _returnvalue_z (+ _returnvalue_z 400.0))))